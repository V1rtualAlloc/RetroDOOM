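; BP_PlayerWeaponBase is a base player weapon that displays the weapon as a flipbook and handles its movement bob.
; A SceneCaptureComponent2D captures only the flipbook, which InitializeWeapon sets and hides in game.
; WeaponBobbing plays the WeaponBob sequence while moving, otherwise stops it and interpolates the flipbook back to the relative location cached at BeginPlay.
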(event `self.ReceiveBeginPlay`
  (`SceneCaptureComponent.ShowOnlyComponent` (`self.SceneCaptureComponent2D`) (`self.Weapon Flipbook`))
  (set `self.Weapon Position` (`SceneComponent.RelativeLocation` (`self.Weapon Flipbook`))))

(event `/Game/Blueprints/IPlayerWeapon.Initialize Weapon`
  (bind _weapon_flipbook (`self.Weapon Flipbook`))
  (`PaperFlipbookComponent.SetFlipbook` _weapon_flipbook null)
  (`SceneComponent.SetHiddenInGame` _weapon_flipbook true false))

(event `Weapon Bobbing`
  (params (`Is Moving` :type Boolean) (`Delta Time` :type "Float (double-precision)"))
  (bind _weapon_flipbook (`self.Weapon Flipbook`))
  (bind _sequenceplayer (`ActorSequenceComponent.SequencePlayer` (`self.Weapon Bob`)))
  (if `Is Moving`
    (`MovieSceneSequencePlayer.Play` _sequenceplayer)
    (else
      (`MovieSceneSequencePlayer.Stop` _sequenceplayer)
      (`SceneComponent.K2_SetRelativeLocation` _weapon_flipbook (`KismetMathLibrary.VInterpTo` (`SceneComponent.RelativeLocation` _weapon_flipbook) (`self.Weapon Position`) `Delta Time` 10.0) false false))))

(fn `UserConstructionScript`)