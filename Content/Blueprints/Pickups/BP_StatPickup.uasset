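; Stat pickup that represents either armor or health in a small or large size, shown as a Paper2D flipbook.
; The construction script sets the flipbook, scale and matching pickup gameplay tag from its type and size.
; Two helper functions read an Ability System attribute and add or remove Player full-health or full-armor tags on the pickup's tag variable, depending on whether the value equals 100.
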(fn `Full Armor Check`
  (params (`Ability System` :type "AbilitySystemComponent Object Reference"))
  (bind _pickup_tag (`self.Pickup Tag`))
  (if (== (`.ReturnValue` (`AbilitySystemBlueprintLibrary.GetFloatAttributeFromAbilitySystemComponent` `Ability System` (struct :`AttributeName` "Armor" :`Attribute` "/Script/RetroDOOM.RetroFPSAttributeSet:Armor"))) 100.0)
    (`BlueprintGameplayTagLibrary.AddGameplayTag` _pickup_tag (struct :`TagName` "Player.Armor.Full"))
    (else
      (`BlueprintGameplayTagLibrary.RemoveGameplayTag` _pickup_tag (struct :`TagName` "Player.Armor.Full")))))

(fn `Full Health Check`
  (params (`Ability System` :type "AbilitySystemComponent Object Reference"))
  (bind _pickup_tag (`self.Pickup Tag`))
  (if (== (`.ReturnValue` (`AbilitySystemBlueprintLibrary.GetFloatAttributeFromAbilitySystemComponent` `Ability System` (struct :`AttributeName` "Health" :`Attribute` "/Script/RetroDOOM.RetroFPSAttributeSet:Health"))) 100.0)
    (`BlueprintGameplayTagLibrary.AddGameplayTag` _pickup_tag (struct :`TagName` "Player.Health.Full"))
    (else
      (`BlueprintGameplayTagLibrary.RemoveGameplayTag` _pickup_tag (struct :`TagName` "Player.Health.Full")))))

(fn `Set Stat Pickup Flipbook`
  (bind _item (`self.Item`))
  (bind _item_2 (`self.Item`))
  (switch `/Game/Blueprints/ENUMs/ENUM_PickupType` (`self.Pickup Type`)
    (:`NewEnumerator0`
      (`PaperFlipbookComponent.SetFlipbook` _item "/Game/Flipbooks/Pickups/FB_Armor_Pickup.FB_Armor_Pickup")
      (switch `/Game/Blueprints/ENUMs/ENUM_PickupSize` (`self.Pickup Size`)
        (:`NewEnumerator0`
          (`SceneComponent.SetRelativeScale3D` _item_2 (1.0 1.0 1.0))
          (set `self.Pickup Tag` (struct :`GameplayTags` (struct :`(TagName` "Pickup.Armor.Small")))))
        (:`NewEnumerator1`
          (`SceneComponent.SetRelativeScale3D` _item_2 (2.0 2.0 2.0))
          (set `self.Pickup Tag` (struct :`GameplayTags` (struct :`(TagName` "Pickup.Armor.Large")))))))
    (:`NewEnumerator1`
      (`PaperFlipbookComponent.SetFlipbook` _item "/Game/Flipbooks/Pickups/FB_Health_Pickup.FB_Health_Pickup")
      (switch `/Game/Blueprints/ENUMs/ENUM_PickupSize` (`self.Pickup Size`)
        (:`NewEnumerator0`
          (`SceneComponent.SetRelativeScale3D` _item_2 (1.0 1.0 1.0))
          (set `self.Pickup Tag` (struct :`GameplayTags` (struct :`(TagName` "Pickup.Health.Small")))))
        (:`NewEnumerator1`
          (`SceneComponent.SetRelativeScale3D` _item_2 (2.0 2.0 2.0))
          (set `self.Pickup Tag` (struct :`GameplayTags` (struct :`(TagName` "Pickup.Health.Large")))))))))

(fn `UserConstructionScript`
  (`parent.UserConstructionScript`)
  (`self.Set Stat Pickup Flipbook`))