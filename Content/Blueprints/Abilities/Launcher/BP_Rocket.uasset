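; BP_Rocket is the launcher ability's projectile, drawn as a Paper2D sprite that yaws toward the player camera each tick.
; When ProjectileMovement stops on an enemy, it applies GE_PlayerLauncherDamage through that enemy's own ability system component, as both source and target.
; On any stop, it spawns BP_RocketExplosion at the impact point, oriented to the surface normal, then destroys itself.
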(event `self.ReceiveTick`
  (params (DeltaSeconds :type "Float (single-precision)"))
  (bind _papersprite (`self.PaperSprite`))
  (bind (_returnvalue_roll _returnvalue_pitch _returnvalue_yaw) (`KismetMathLibrary.BreakRotator` (`KismetMathLibrary.FindLookAtRotation` (`SceneComponent.K2_GetComponentLocation` _papersprite) (`PlayerCameraManager.GetCameraLocation` (`GameplayStatics.GetPlayerCameraManager` 0)))))
  (`SceneComponent.K2_SetWorldRotation` _papersprite (`KismetMathLibrary.MakeRotator` 0.0 0.0 (- _returnvalue_yaw 90.0)) false false))

(event `self.ProjectileMovement.OnProjectileStop`
  (params (ImpactResult :type "HitResult Structure (by ref)"))
  (bind _asbp_enemy (cast `/Game/Blueprints/Enemies/BP_Enemy` ImpactResult_HitActor)
    (:`then`
      (bind _returnvalue (`AbilitySystemBlueprintLibrary.GetAbilitySystemComponent` _asbp_enemy))
      (`AbilitySystemComponent.BP_ApplyGameplayEffectToTarget` _returnvalue "/Game/Blueprints/Abilities/Launcher/GE_PlayerLauncherDamage.GE_PlayerLauncherDamage_C" _returnvalue 0.0 (`AbilitySystemComponent.MakeEffectContext` _returnvalue)))
    (:`CastFailed`
      _))
  (`|SpawnActorFromClass` "/Game/Blueprints/Abilities/Launcher/BP_RocketExplosion.BP_RocketExplosion_C" (`KismetMathLibrary.MakeTransform` ImpactResult_ImpactPoint (`KismetMathLibrary.Conv_VectorToRotator` ImpactResult_ImpactNormal)) "Undefined" "OverrideRootScale" null null)
  (`self.K2_DestroyActor`))

(fn `UserConstructionScript`)