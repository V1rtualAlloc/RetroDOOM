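; Enemy pistol ability that fires a hitscan shot from a BP_OutleaderEnemy at the RetroFPSCharacter.
; On FireWeapon, it caches the owning enemy, then runs a Visibility line trace from the capsule along its forward vector out to WeaponRange.
; If the hit actor is a RetroFPSCharacter, it applies an effect with the enemy as instigator.
; The trace leaves persistent debug drawing on.
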(event `self.Fire Weapon`
  (`self.Get Enemy`)
  (bind _actor (`self.Get Line Trace`))
  (bind _asretro_fpscharacter (cast `RetroFPSCharacter` _actor))
  (`self.Apply Effect` (`self.Pistol Enemy`) _asretro_fpscharacter))

(fn `Get Enemy`
  (bind _returnvalue_owneractor (break `GameplayAbilityActorInfo` (`self.GetActorInfo`)))
  (`/Engine/EditorBlueprintResources/StandardMacros.IsValid` (`self.Pistol Enemy`)
    (:`Is Valid`
      _)
    (:`Is Not Valid`
      (bind _asbp_outleader_enemy (cast `/Game/Blueprints/Enemies/BP_OutleaderEnemy` _returnvalue_owneractor))
      (set `self.Pistol Enemy` _asbp_outleader_enemy)))
  (return))

(fn `Get Line Trace`
  (returns (Actor :type "Actor Object Reference"))
  (bind _capsulecomponent (`Character.CapsuleComponent` (`self.Pistol Enemy`)))
  (bind _returnvalue (`SceneComponent.K2_GetComponentLocation` _capsulecomponent))
  (bind _outhit (`KismetSystemLibrary.LineTraceSingle` :`Start` _returnvalue :`End` (+ _returnvalue (* (`KismetMathLibrary.GetForwardVector` (`SceneComponent.K2_GetComponentRotation` _capsulecomponent)) (`self.Weapon Range`))) :`TraceChannel` "TraceTypeQuery1" :`DrawDebugType` "Persistent"))
  (bind (_bblockinghit _binitialoverlap _time _distance _location _impactpoint _normal _impactnormal _physmat _hitactor) (`GameplayStatics.BreakHitResult` _outhit))
  (`/Engine/EditorBlueprintResources/StandardMacros.IsValid` _hitactor
    (:`Is Valid`
      (return _hitactor))))