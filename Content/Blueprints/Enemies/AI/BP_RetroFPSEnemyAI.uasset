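; AI logic for retro FPS enemies that turns perception updates on Player-tagged actors into blackboard state.
; Sensing the player sets the line-of-sight flag and target actor, and cancels any pending lost-sight timer.
; Losing the player clears the flag at once but keeps the target for a grace period, after which a timer clears it.
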(event `self.AIPerception.OnTargetPerceptionUpdated`
  (params (Actor :type "Actor Object Reference") (Stimulus :type "AIStimulus Structure"))
  (bind _output_get (set `self.Perceived Actor` Actor))
  (if (`self.ActorHasTag` _output_get "Player")
    (if Stimulus_bSuccessfullySensed
      (`KismetSystemLibrary.K2_ClearAndInvalidateTimerHandle` (`self.Lost Sight Timer`))
      (`self.Update Sight Key` true)
      (`self.Update Target Key` (`self.Perceived Actor`))
      (else
        (bind _returnvalue (`KismetSystemLibrary.K2_SetTimerDelegate` (delegate `Lost Sight`) 8.0))
        (set `self.Lost Sight Timer` _returnvalue)
        (`self.Update Sight Key` false)))))

(event `Lost Sight`
  (`self.Update Target Key` null))

(fn `Update Sight Key`
  (params (`Has Line of Sight` :type Boolean))
  (`BlackboardComponent.SetValueAsBool` (`AIBlueprintHelperLibrary.GetBlackboard` null) "Can See Target" `Has Line of Sight`))

(fn `Update Target Key`
  (params (`Target Actor` :type "Actor Object Reference"))
  (`BlackboardComponent.SetValueAsObject` (`AIBlueprintHelperLibrary.GetBlackboard` null) "Target Actor" `Target Actor`))

(fn `UserConstructionScript`)