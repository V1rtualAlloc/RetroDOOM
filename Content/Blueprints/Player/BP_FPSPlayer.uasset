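; BP_FPSPlayer is the first-person player character, handling movement, mouse look, weapon equipping and HUD creation.
; On BeginPlay it adds WBP_HUD and equips BP_PlayerWeaponBase through a Child Actor component, initializing it via IPlayerWeapon and playing its draw sequence.
; Tick drives weapon bobbing from movement velocity.
; Fire input activates Gameplay Ability System abilities by tag instead of calling the weapon directly.
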(event `self.ReceiveBeginPlay`
  (`parent.ReceiveBeginPlay`)
  (bind _returnvalue (`|CreateWidget` "/Game/Blueprints/Widgets/WBP_HUD.WBP_HUD_C"))
  (`UserWidget.AddToViewport` _returnvalue 0)
  (`self.Equip Weapon` "/Game/Blueprints/Player/BP_PlayerWeaponBase.BP_PlayerWeaponBase_C"))

(event `InputAxis|HorizontalMovement`
  (params (AxisValue :type "Float (single-precision)"))
  (bind (_returnvalue_roll _returnvalue_pitch _returnvalue_yaw) (`KismetMathLibrary.BreakRotator` (`self.GetControlRotation`)))
  ;[0 0 0] Movement
  (`self.AddMovementInput` (`KismetMathLibrary.GetRightVector` (`KismetMathLibrary.MakeRotator` 0.0 0.0 _returnvalue_yaw)) AxisValue))

(event `InputAxis|VerticalMovement`
  (params (AxisValue :type "Float (single-precision)"))
  (bind (_returnvalue_roll _returnvalue_pitch _returnvalue_yaw) (`KismetMathLibrary.BreakRotator` (`self.GetControlRotation`)))
  ;[0 0 0] Movement
  (`self.AddMovementInput` (`KismetMathLibrary.GetForwardVector` (`KismetMathLibrary.MakeRotator` 0.0 0.0 _returnvalue_yaw)) AxisValue))

(event `self.ReceiveTick`
  (params (DeltaSeconds :type "Float (single-precision)"))
  (bind _asbp_player_weapon_base (cast `/Game/Blueprints/Player/BP_PlayerWeaponBase` (`ChildActorComponent.ChildActor` (`self.Weapon`))))
  (`/Game/Blueprints/Player/BP_PlayerWeaponBase.Weapon Bobbing` _asbp_player_weapon_base (> (`KismetMathLibrary.VSize` (`MovementComponent.Velocity` (`self.CharacterMovement`))) 0.0) DeltaSeconds))

(event `InputAxis|MouseLookHorizontal`
  (params (AxisValue :type "Float (single-precision)"))
  ;[0 0 0] Mouse Look
  (`self.AddControllerYawInput` AxisValue))

(event `InputAxis|MouseLookVertical`
  (params (AxisValue :type "Float (single-precision)"))
  ;[0 0 0] Mouse Look
  (`self.AddControllerPitchInput` AxisValue))

(event `Equip Weapon`
  (params (Weapon :type "/Game/Blueprints/Player/BP_PlayerWeaponBase Class Reference"))
  (bind _weapon (`self.Weapon`))
  (bind _childactor (`ChildActorComponent.ChildActor` _weapon))
  ;[0 0 0] Equip Weapon
  (bind _output_get (set `self.Current Weapon` Weapon))
  (`ChildActorComponent.SetChildActorClass` _weapon _output_get)
  (if (`KismetSystemLibrary.DoesImplementInterface` _childactor "/Game/Blueprints/Interfaces/IPlayerWeapon.IPlayerWeapon_C")
    (message `/Game/Blueprints/Interfaces/IPlayerWeapon.Initialize Weapon` _childactor)
    (bind _asbp_player_weapon_base (cast `/Game/Blueprints/Player/BP_PlayerWeaponBase` _childactor))
    (`MovieSceneSequencePlayer.Play` (`ActorSequenceComponent.SequencePlayer` (`/Game/Blueprints/Player/BP_PlayerWeaponBase.Weapon Draw` _asbp_player_weapon_base)))))

(event `InputAction|FireWeapon`
  (params (Key :type "Key Structure"))
  (:`Pressed`
    (`AbilitySystemComponent.TryActivateAbilitiesByTag` (`self.AbilitySystemComponent`) (`self.Gameplay Tag Container`) false)))

(fn `UserConstructionScript`)