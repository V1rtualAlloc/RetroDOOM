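; BP_Launcher is a rocket launcher weapon for the FPS player, drawn with flipbook animations.
; InitializeWeapon shows the idle flipbook and caches the BP_FPSPlayer pawn.
; ShootLauncher flashes a point light, refreshes the player's UI, spawns a BP_Rocket at the spawn point, and plays the fire flipbook for its length before returning to idle.
; A sound playback node is present but unconnected.
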(event `/Game/Blueprints/Interfaces/IPlayerWeapon.Initialize Weapon`
  ;[0 0 0] Equip Weapon
  (`PaperFlipbookComponent.SetFlipbook` (`self.Weapon Flipbook`) (`self.Idle Launcher`))
  (`SceneComponent.SetHiddenInGame` (`self.Weapon Flipbook`) false false)
  (bind _asbp_fpsplayer (cast `/Game/Blueprints/Player/BP_FPSPlayer` (`GameplayStatics.GetPlayerPawn` 0)))
  (set `self.Player` _asbp_fpsplayer))

(event `Shoot Launcher`
  (bind _weapon_flipbook (`self.Weapon Flipbook`))
  ;[0 0 0] Launcher Fire Animation
  (`self.Light Flash`)
  (`/Game/Blueprints/Player/BP_FPSPlayer.Update UI` (`self.Player`))
  (`|SpawnActorFromClass` "/Game/Blueprints/Abilities/Launcher/BP_Rocket.BP_Rocket_C" (`SceneComponent.K2_GetComponentToWorld` (`self.Rocket Spawn Point`)) "Undefined" "OverrideRootScale" null null)
  (`PaperFlipbookComponent.SetFlipbook` _weapon_flipbook (`self.Fire Launcher`))
  (`KismetSystemLibrary.Delay` (`PaperFlipbookComponent.GetFlipbookLength` _weapon_flipbook))
  (`PaperFlipbookComponent.SetFlipbook` (`self.Weapon Flipbook`) (`self.Idle Launcher`)))

(event `Light Flash`
  (bind _pointlight (`self.PointLight`))
  ;[0 0 0] Light Flash
  (`SceneComponent.SetHiddenInGame` _pointlight false false)
  (`KismetSystemLibrary.Delay` 0.25)
  (`SceneComponent.SetHiddenInGame` _pointlight true false))

(fn `UserConstructionScript`
  (`parent.UserConstructionScript`))